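; Player controller for the main menu that creates the menu widget and handles keyboard changes to display settings.
; On BeginPlay it adds MainMenuWidget to the viewport and keeps a reference to it.
; A and D step the widget's resolution or display mode index down or up, depending on its Selected text.
; The widget's own functions then apply the change: text and command for resolution, a mode change for display mode.
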(event `Key|W`
  (params (Key :type "Key Structure" :default "AnyKey")))

(event `Key|S`
  (params (Key :type "Key Structure" :default "AnyKey")))

(event `self.ReceiveBeginPlay`
  (bind _returnvalue (`|CreateWidget` "/Game/UI/Menus/MainMenuWidget.MainMenuWidget_C"))
  (set `self.MainMenuReference` _returnvalue)
  (`UserWidget.AddToViewport` _returnvalue 0))

(event `Key|Enter`
  (params (Key :type "Key Structure" :default "AnyKey")))

(event `self.ReceiveTick`
  (params (DeltaSeconds :type "Float (single-precision)")))

(event `Key|A`
  (params (Key :type "Key Structure" :default "AnyKey"))
  (bind _mainmenureference (`self.MainMenuReference`))
  (bind _mainmenureference_2 (`self.MainMenuReference`))
  ;[1 1 1] Keyboard input for resolution change
  (:`Pressed`
    (if (`KismetTextLibrary.EqualEqual_TextText` (`/Game/UI/Menus/MainMenuWidget.Selected` _mainmenureference_2) (`|FormatText` "resolution"))
      (bind _output_get (set `/Game/UI/Menus/MainMenuWidget.CurrentResolution` (+ (`/Game/UI/Menus/MainMenuWidget.CurrentResolution` _mainmenureference_2) -1) _mainmenureference_2))
      (`/Game/UI/Menus/MainMenuWidget.ChangeResolutionText` _mainmenureference _output_get)
      (`/Game/UI/Menus/MainMenuWidget.SetResolutionCommand` _mainmenureference _output_get))))

(event `Key|D`
  (params (Key :type "Key Structure" :default "AnyKey"))
  (bind _mainmenureference (`self.MainMenuReference`))
  (bind _mainmenureference_2 (`self.MainMenuReference`))
  ;[1 1 1] Keyboard input for resolution change
  (:`Pressed`
    (if (`KismetTextLibrary.EqualEqual_TextText` (`/Game/UI/Menus/MainMenuWidget.Selected` _mainmenureference) (`|FormatText` "resolution"))
      (bind _output_get (set `/Game/UI/Menus/MainMenuWidget.CurrentResolution` (+ (`/Game/UI/Menus/MainMenuWidget.CurrentResolution` _mainmenureference) 1) _mainmenureference))
      (`/Game/UI/Menus/MainMenuWidget.ChangeResolutionText` _mainmenureference_2 _output_get)
      (`/Game/UI/Menus/MainMenuWidget.SetResolutionCommand` _mainmenureference_2 _output_get))))

(event `Key|A`
  (params (Key :type "Key Structure" :default "AnyKey"))
  (bind _mainmenureference (`self.MainMenuReference`))
  ;[1 1 1] Keyboard input for displaymode
  (:`Pressed`
    (if (`KismetTextLibrary.EqualEqual_TextText` (`/Game/UI/Menus/MainMenuWidget.Selected` _mainmenureference) (`|FormatText` "displaymode"))
      (bind _output_get (set `/Game/UI/Menus/MainMenuWidget.CurrentDisplayMode` (+ (`/Game/UI/Menus/MainMenuWidget.CurrentDisplayMode` _mainmenureference) -1) _mainmenureference))
      (`/Game/UI/Menus/MainMenuWidget.ChangeDisplayMode` (`self.MainMenuReference`) _output_get))))

(event `Key|D`
  (params (Key :type "Key Structure" :default "AnyKey"))
  (bind _mainmenureference (`self.MainMenuReference`))
  ;[1 1 1] Keyboard input for displaymode
  (:`Pressed`
    (if (`KismetTextLibrary.EqualEqual_TextText` (`/Game/UI/Menus/MainMenuWidget.Selected` _mainmenureference) (`|FormatText` "displaymode"))
      (bind _output_get (set `/Game/UI/Menus/MainMenuWidget.CurrentDisplayMode` (+ (`/Game/UI/Menus/MainMenuWidget.CurrentDisplayMode` _mainmenureference) 1) _mainmenureference))
      (`/Game/UI/Menus/MainMenuWidget.ChangeDisplayMode` (`self.MainMenuReference`) _output_get))))

(fn `UserConstructionScript`)