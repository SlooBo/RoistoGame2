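; Debug gas trap that continuously damages the player while an overlap is active.
; Begin and end overlap events print debug strings and toggle a PlayerOverlap flag without checking which actor overlaps.
; While the flag is set, Tick casts player pawn 0 to Player and calls TakeDamage with a fixed amount every frame, so damage scales with frame rate.
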(event `self.ReceiveBeginPlay`)

(event `self.ReceiveActorBeginOverlap`
  (params (OtherActor :type "Actor Object Reference"))
  (`KismetSystemLibrary.PrintString` "overlap begin")
  (set `self.PlayerOverlap` true))

(event `self.ReceiveActorEndOverlap`
  (params (OtherActor :type "Actor Object Reference"))
  (`KismetSystemLibrary.PrintString` "overlapend")
  (set `self.PlayerOverlap` false))

(event `self.ReceiveTick`
  (params (DeltaSeconds :type "Float (single-precision)"))
  (if (`self.PlayerOverlap`)
    (bind _asplayer (cast `/Game/Blueprints/Player/Player` (`GameplayStatics.GetPlayerPawn` 0)))
    (`/Game/Blueprints/Player/Player.TakeDamage` _asplayer 5.0)))

(fn `UserConstructionScript`)