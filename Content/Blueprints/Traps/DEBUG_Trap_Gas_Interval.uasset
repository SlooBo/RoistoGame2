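; Debug gas trap that damages the player while its gas is active and something overlaps it.
; Overlap events print debug text and set a flag without checking which actor entered or left.
; Tick applies fixed damage to player pawn 0 every frame while both flags are set, so damage scales with frame rate.
; Tick-driven Delay nodes alternate the Gas component and Active flag every three seconds.
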(event `self.ReceiveBeginPlay`)

(event `/Game/Blueprints/Traps/DEBUG_Trap_Gas_Constant.ReceiveActorBeginOverlap`
  (params (OtherActor :type "Actor Object Reference"))
  (`KismetSystemLibrary.PrintString` "overlap begin")
  (set `self.PlayerOverlap` true))

(event `self.ReceiveActorEndOverlap`
  (params (OtherActor :type "Actor Object Reference"))
  (`KismetSystemLibrary.PrintString` "overlapend")
  (set `self.PlayerOverlap` false))

(event `/Game/Blueprints/Traps/DEBUG_Trap_Gas_Constant.ReceiveTick`
  (params (DeltaSeconds :type "Float (single-precision)"))
  (`|ExecutionSequence`
    (:`then_0`
      (if (`self.Active`)
        (if (`self.PlayerOverlap`)
          (bind _asplayer (cast `/Game/Blueprints/Player/Player` (`GameplayStatics.GetPlayerPawn` 0)))
          (`/Game/Blueprints/Player/Player.TakeDamage` _asplayer 5.0))))
    (:`then_1`
      (if (`self.Active`)
        (`KismetSystemLibrary.Delay` 3.0)
        (`ActorComponent.SetActive` (`self.Gas`) false true)
        (set `self.Active` false)
        (else
          (`KismetSystemLibrary.Delay` 3.0)
          (`ActorComponent.SetActive` (`self.Gas`) true true)
          (set `self.Active` true))))))

(fn `UserConstructionScript`)