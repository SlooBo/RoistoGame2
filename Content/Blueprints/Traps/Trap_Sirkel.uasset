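; Trap actor with three groups of spinning "Sirkels" on holders that slide back and forth, with sparks on contact.
; Tick rotates the sirkels and offsets each holder along local Z, with the middle moving opposite to the outer two.
; A Switch flag and one-second Delays on Tick reverse the speeds, making movement frame-rate dependent.
; Three colliders each toggle their own spark effect on overlap; no damage is applied here.
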(event `self.ReceiveBeginPlay`
  (`ActorComponent.Deactivate` (`self.Sparks`)))

(event `self.ReceiveActorBeginOverlap`
  (params (OtherActor :type "Actor Object Reference")))

(event `self.ReceiveTick`
  (params (DeltaSeconds :type "Float (single-precision)"))
  (bind _speedouter (`self.SpeedOuter`))
  (`SceneComponent.K2_AddLocalRotation` (`self.sirkels_right`) (struct :`Pitch` -15.0) false false)
  (`SceneComponent.K2_AddLocalRotation` (`self.sirkels_mid`) (struct :`Pitch` -15.0) false false)
  (`SceneComponent.K2_AddLocalRotation` (`self.sirkels_left`) (struct :`Pitch` -15.0) false false)
  (`|ExecutionSequence`
    (:`then_0`
      (`self.Move` (`self.sirkel_holder_mid`) (`self.SpeedInner`)))
    (:`then_1`
      (`self.Move` (`self.sirkel_holder_right`) _speedouter))
    (:`then_2`
      (`self.Move` (`self.sirkel_holder_left`) _speedouter))
    (:`then_3`
      (if (`self.switch`)
        (`KismetSystemLibrary.Delay` 1.0)
        (set `self.SpeedInner` -0.5)
        (set `self.SpeedOuter` 0.5)
        (set `self.switch` false)
        (else
          (`KismetSystemLibrary.Delay` 1.0)
          (set `self.SpeedInner` 0.5)
          (set `self.SpeedOuter` -0.5)
          (set `self.switch` true))))))

(event `self.Collider.OnComponentBeginOverlap`
  (params (OtherActor :type "Actor Object Reference") (OtherComp :type "PrimitiveComponent Object Reference") (OtherBodyIndex :type Integer) (bFromSweep :type Boolean) (SweepResult :type "HitResult Structure (by ref)"))
  (`ActorComponent.Activate` (`self.Sparks`) false))

(event `self.Collider.OnComponentEndOverlap`
  (params (OtherActor :type "Actor Object Reference") (OtherComp :type "PrimitiveComponent Object Reference") (OtherBodyIndex :type Integer))
  (`ActorComponent.Deactivate` (`self.Sparks`)))

(event `self.Collider3.OnComponentBeginOverlap`
  (params (OtherActor :type "Actor Object Reference") (OtherComp :type "PrimitiveComponent Object Reference") (OtherBodyIndex :type Integer) (bFromSweep :type Boolean) (SweepResult :type "HitResult Structure (by ref)"))
  (`ActorComponent.Activate` (`self.Sparks3`) false))

(event `self.Collider3.OnComponentEndOverlap`
  (params (OtherActor :type "Actor Object Reference") (OtherComp :type "PrimitiveComponent Object Reference") (OtherBodyIndex :type Integer))
  (`ActorComponent.Deactivate` (`self.Sparks3`)))

(event `self.Collider2.OnComponentBeginOverlap`
  (params (OtherActor :type "Actor Object Reference") (OtherComp :type "PrimitiveComponent Object Reference") (OtherBodyIndex :type Integer) (bFromSweep :type Boolean) (SweepResult :type "HitResult Structure (by ref)"))
  (`ActorComponent.Activate` (`self.Sparks2`) false))

(event `self.Collider2.OnComponentEndOverlap`
  (params (OtherActor :type "Actor Object Reference") (OtherComp :type "PrimitiveComponent Object Reference") (OtherBodyIndex :type Integer))
  (`ActorComponent.Deactivate` (`self.Sparks2`)))

(fn `Move`
  (params (staticmeshactor :type "StaticMeshComponent Object Reference") (movespeed :type "Float (double-precision)"))
  (`SceneComponent.K2_AddLocalOffset` staticmeshactor (`KismetMathLibrary.MakeVector` 0.0 0.0 movespeed) false false))

(fn `UserConstructionScript`)