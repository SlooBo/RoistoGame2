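; Debug tower projectile: a nuclear bomb that explodes on overlap and deals area damage to the player.
; Tick turns the bomb mesh toward the player and starts a ten-second delayed self-destruct.
; Sphere overlap fires the explosion, removes the bomb and movement, damages the player if inside AoE, then clears the trail and actor after delays.
; Crater decal placement by downward trace is disconnected, so the crater stays hidden.
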(event `self.ReceiveBeginPlay`
  (`SceneComponent.SetVisibility` (`self.Crater`) false false))

(event `self.ReceiveActorBeginOverlap`
  (params (OtherActor :type "Actor Object Reference")))

(event `self.Sphere.OnComponentBeginOverlap`
  (params (OtherActor :type "Actor Object Reference") (OtherComp :type "PrimitiveComponent Object Reference") (OtherBodyIndex :type Integer) (bFromSweep :type Boolean) (SweepResult :type "HitResult Structure (by ref)"))
  (bind _returnvalue (`GameplayStatics.GetPlayerPawn` 0))
  (`|ExecutionSequence`
    (:`then_0`
      (`ActorComponent.Activate` (`self.P_Explosion`) false)
      (set `self.IsDestroyed` true)
      (`ActorComponent.K2_DestroyComponent` (`self.ProjectileMovement`))
      (`ActorComponent.K2_DestroyComponent` (`self.Sphere`))
      (`ActorComponent.K2_DestroyComponent` (`self.nuclearBomb`))
      (`KismetSystemLibrary.Delay` 1.0)
      (`ActorComponent.K2_DestroyComponent` (`self.Trail`))
      (`KismetSystemLibrary.Delay` 10.0)
      (`self.K2_DestroyActor`))
    (:`then_1`
      (if (`PrimitiveComponent.IsOverlappingActor` (`self.AoE`) _returnvalue)
        (bind _asplayer (cast `/Game/Blueprints/Player/Player` _returnvalue))
        (`/Game/Blueprints/Player/Player.TakeDamage` _asplayer 10.0)))))

(event `/Game/Blueprints/Towers/DEBUG_Bullet1.ReceiveTick`
  (params (DeltaSeconds :type "Float (single-precision)"))
  (if (not (`self.IsDestroyed`))
    (`SceneComponent.K2_SetRelativeRotation` (`self.nuclearBomb`) (`KismetMathLibrary.MakeRotator` (.roll (`KismetMathLibrary.FindLookAtRotation` (`self.K2_GetActorLocation`) (`self.K2_GetActorLocation` (`GameplayStatics.GetPlayerPawn` 0)))) (- (.pitch (`KismetMathLibrary.FindLookAtRotation` (`self.K2_GetActorLocation`) (`self.K2_GetActorLocation` (`GameplayStatics.GetPlayerPawn` 0)))) 90.0) (.yaw (`KismetMathLibrary.FindLookAtRotation` (`self.K2_GetActorLocation`) (`self.K2_GetActorLocation` (`GameplayStatics.GetPlayerPawn` 0))))) false false)
    (`KismetSystemLibrary.Delay` 10.0)
    (`self.K2_DestroyActor`)))

(fn `UserConstructionScript`)