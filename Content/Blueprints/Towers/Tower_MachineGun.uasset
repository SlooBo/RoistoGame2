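; Machine gun tower that tracks the player's pawn and fires at it automatically.
; Each Tick aims Cube1 at the pawn, applying the world-space look-at as a relative rotation.
; A Delay on Tick acts as the ShootCD cooldown before each call to Shoot.
; Shoot spawns a DEBUG_Bullet1 at Cube1's location, oriented toward the pawn, with no range or line-of-sight check.
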(event `self.ReceiveBeginPlay`)

(event `self.ReceiveActorBeginOverlap`
  (params (OtherActor :type "Actor Object Reference")))

(event `self.ReceiveTick`
  (params (DeltaSeconds :type "Float (single-precision)"))
  (`SceneComponent.K2_SetRelativeRotation` (`self.Cube1`) (`KismetMathLibrary.FindLookAtRotation` (`SceneComponent.K2_GetComponentLocation` (`self.Cube1`)) (`self.K2_GetActorLocation` (`Controller.K2_GetPawn` (`GameplayStatics.GetPlayerController` 0)))) false false)
  (`KismetSystemLibrary.Delay` (`self.ShootCD`))
  (`self.Shoot`))

(fn `Shoot`
  (`|SpawnActorFromClass` "/Game/Blueprints/Towers/DEBUG_Bullet1.DEBUG_Bullet1_C" (`KismetMathLibrary.MakeTransform` (`SceneComponent.K2_GetComponentLocation` (`self.Cube1`)) (`KismetMathLibrary.FindLookAtRotation` (`SceneComponent.K2_GetComponentLocation` (`self.Cube1`)) (`self.K2_GetActorLocation` (`Controller.K2_GetPawn` (`GameplayStatics.GetPlayerController` 0))))) "Undefined" "OverrideRootScale"))

(fn `UserConstructionScript`)