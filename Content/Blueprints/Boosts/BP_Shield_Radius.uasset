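; BP_Shield_Radius is a short-lived shield actor that drives a shrinking radius effect through the MAT_Shield_PARAMS material parameter collection.
; Construction scales its Sphere component by Radius and writes the actor's location to the collection.
; Tick republishes the location, lowers Radius by a fixed per-frame step independent of delta time, and writes it to the collection.
; A Delay on Tick destroys the actor after one second.
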(event `self.ReceiveBeginPlay`)

(event `self.ReceiveActorBeginOverlap`
  (params (OtherActor :type "Actor Object Reference")))

(event `self.ReceiveTick`
  (params (DeltaSeconds :type "Float (single-precision)"))
  (`KismetMaterialLibrary.SetVectorParameterValue` "/Game/Materials/Boosts/MAT_Shield_PARAMS.MAT_Shield_PARAMS" "Location" (`KismetMathLibrary.Conv_VectorToLinearColor` (`self.K2_GetActorLocation`)))
  (bind _output_get (set `self.Radius` (- (`self.Radius`) 25.0)))
  (`KismetMaterialLibrary.SetScalarParameterValue` "/Game/Materials/Boosts/MAT_Shield_PARAMS.MAT_Shield_PARAMS" "Radius" _output_get)
  (`KismetSystemLibrary.Delay` 1.0)
  (`self.K2_DestroyActor`))

(fn `UserConstructionScript`
  (`SceneComponent.SetRelativeScale3D` (`self.Sphere`) (`KismetMathLibrary.Conv_DoubleToVector` (`self.Radius`)))
  (`KismetMaterialLibrary.SetVectorParameterValue` "/Game/Materials/Boosts/MAT_Shield_PARAMS.MAT_Shield_PARAMS" "Location" (`KismetMathLibrary.Conv_VectorToLinearColor` (`self.K2_GetActorLocation`))))